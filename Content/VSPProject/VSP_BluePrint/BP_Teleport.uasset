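; BP_Teleport is a trigger actor that moves the player to the mirrored position across the world X origin.
; When the player pawn overlaps its Box while Close is false, it negates the pawn's X location and keeps Y and Z.
; It first sets Close on the referenced Teleport to block an immediate bounce back.
; Ending an overlap with the Box clears its own Close flag.
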(event OnComponentBeginOverlap(Box)
  (params (OverlappedComponent :type Primitive%20Component%20Object%20Reference) (OtherActor :type Actor%20Object%20Reference) (OtherComp :type Primitive%20Component%20Object%20Reference) (OtherBodyIndex :type Integer) (bFromSweep :type Boolean) (SweepResult :type Hit%20Result%20Structure%20%28by%20ref%29))
  (bind _returnvalue (Game|Player|GetPlayerPawn 0))
  (bind _returnvalue_2 (Transformation|GetActorLocation _returnvalue))
  (if (== _returnvalue OtherActor)
    (if (not (Variables|Default|GetClose))
      (Variables|BP_Teleport_C|SetClose (Variables|Default|GetTeleport) true)
      (Transformation|SetActorLocation OtherActor (Math|Vector|MakeVector (* (.x _returnvalue_2) -1.0) (.y _returnvalue_2) (.z _returnvalue_2)) false false))))

(event OnComponentEndOverlap(Box)
  (params (OverlappedComponent :type Primitive%20Component%20Object%20Reference) (OtherActor :type Actor%20Object%20Reference) (OtherComp :type Primitive%20Component%20Object%20Reference) (OtherBodyIndex :type Integer))
  (Variables|Default|SetClose false))

(fn ConstructionScript)