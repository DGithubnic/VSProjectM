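; Monster spawner that spawns waves of BP_Monster1 at random positions on a looping timer, raising their level over time.
; Each SpawnMonster call advances a SpawnTime counter, which periodically increments MonsterLevel up to a cap of ten.
; Every spawn takes its stats from the DT_Monster row named after that level.
; Positions are re-rolled through a wire loop-back until they land far enough from the player.
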(event EventBeginPlay
  ;[1 1 1] SpawnMonster 함수를 호출
  (Utilities|Time|SetTimerbyFunctionName 0 "SpawnMonster" 2.0 true))

(fn ConstructionScript)

(fn SpawnMonster
  (Variables|Default|SetSpawnTime (+ (Variables|Default|GetSpawnTime) 5))
  (if (== (Math|Integer|%(Integer) (Variables|Default|GetSpawnTime) 10) 0)
    (if (== (Variables|Default|GetMonsterLevel) 10)
      _
      (else
        (Math|Integer|IncrementInt (Variables|Default|GetMonsterLevel)
          (:%20%20
            _)))))
  (for _index (range 0 4)
    (bind _returnvalue (Utilities|GetDataTableRow "/Game/VSPProject/VSP_Struct/DT_Monster.DT_Monster" (Utilities|String|StringToName (Utilities|String|ToString(Integer) (Variables|Default|GetMonsterLevel))))
      (:then
        (bind _output_get (Variables|Default|SetMonsterPosition (Math|Vector|MakeVector (Math|Random|RandomFloatinRange -5e+03 5e+03) (Math|Random|RandomFloatinRange -1.5e+03 1.5e+03) 6e+01) :!label _label))
        (if (< 1.8e+03 (Math|Vector|Distance(Vector) _output_get (Transformation|GetActorLocation (Game|GetPlayerCharacter 0))))
          (Game|SpawnActorfromClass "/Game/VSPProject/VSP_BluePrint/BP_Monster1.BP_Monster1_C" (Math|Transform|MakeTransform (Variables|Default|GetMonsterPosition) "0, 0, 0" "1,1,1") "Undefined" 0 _returnvalue 0)
          (else
            (goto _label)))))))