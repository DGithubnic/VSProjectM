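; BP_Monster1 is a monster that constantly chases the player character.
; On BeginPlay it caches player 0 as Target and copies mesh, experience, attack, speed and HP from the STMonsterV struct.
; Each Tick it turns toward Target without pitch and offsets itself horizontally along that direction by Speed, unscaled by delta time.
; Experience, attack and HP are only stored here.
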(event EventBeginPlay
  (bind _st_monsterv (Variables|Default|GetST_MonsterV))
  ;[1 1 1] Target에 정보 넣어주기
  (Variables|Default|SetTarget (Game|GetPlayerCharacter 0))
  (Class|SkinnedMeshComponent|SetSkeletalMesh (Variables|Character|GetMesh) (.mesh _st_monsterv) true)
  (Variables|Default|SetExp (.exp _st_monsterv))
  (Variables|Default|SetAttack (.attack _st_monsterv))
  (Variables|Default|SetSpeed (.speed _st_monsterv))
  (Variables|Default|SetHp (.hp _st_monsterv)))

(event EventTick
  (params (DeltaSeconds :type Float%20%28single-precision%29))
  (bind _returnvalue (Transformation|GetActorLocation))
  (bind _returnvalue_2 (Transformation|GetActorLocation))
  (bind _target (Variables|Default|GetTarget))
  (bind _target_2 (Variables|Default|GetTarget))
  (bind _speed (Variables|Default|GetSpeed))
  (bind _returnvalue_3 (Transformation|GetActorLocation _target))
  (bind _returnvalue_4 (Transformation|GetActorLocation _target_2))
  (bind _returnvalue_5 (Math|Rotator|FindLookatRotation _returnvalue_2 _returnvalue_4))
  (bind _returnvalue_6 (Math|Rotator|FindLookatRotation _returnvalue _returnvalue_3))
  (bind _returnvalue_7 (Math|Vector|GetForwardVector _returnvalue_6))
  ;[1 1 1] 몬스터가 플레이어를 따라가기
  (Transformation|SetActorRotation (Math|Rotator|MakeRotator (.roll _returnvalue_5) 0.0 (.yaw _returnvalue_5)))
  (Transformation|AddActorWorldOffset (Math|Vector|MakeVector (* _speed (.x _returnvalue_7)) (* _speed (.y _returnvalue_7)) 0.0)))

(fn ConstructionScript)